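; BP_CGPlayer is the player actor that switches its camera between a front view and a top view.
; On BeginPlay it binds to CGGameMode events, using the top view during container placement and inspection and returning to front view when either ends.
; Each switch saves the current location for that view and jumps to the other's saved one, while a timeline plays or reverses to animate camera pitch.
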(event Custom|OnStartPlacingContainer_事件_0
  (params (NewUnit :type Unit%20Object%20Reference))
  (CallFunction|SwitchtoTopView))

(event Custom|SwitchToTopView
  (Variables|Default|SetFrontViewLocation (Transformation|GetActorLocation))
  (Transformation|SetActorLocation (Variables|Default|GetTopViewLocation) false false)
  (bind _camerapitchangle (Timeline|CameraRotation Play)
    (:Update
      (Transformation|SetWorldRotation (Variables|Default|GetCamera) (Math|Rotator|MakeRotator 0.0 _camerapitchangle 0.0) false false))))

(event Custom|SwitchToFrontView
  (Variables|Default|SetTopViewLocation (Transformation|GetActorLocation))
  (Transformation|SetActorLocation (Variables|Default|GetFrontViewLocation) false false)
  (bind _camerapitchangle (Timeline|CameraRotation Reverse)
    (:Update
      (Transformation|SetWorldRotation (Variables|Default|GetCamera) (Math|Rotator|MakeRotator 0.0 _camerapitchangle 0.0) false false))))

(event Custom|OnEndPlacingContainer_事件_0
  (params (bSuccessful :type Boolean) (Cost :type Integer) (NewUnit :type Unit%20Object%20Reference))
  (CallFunction|SwitchtoFrontView))

(event Custom|OnStartInspection_事件_0
  (CallFunction|SwitchtoTopView))

(event Custom|OnEndInspection_事件_0
  (CallFunction|SwitchtoFrontView))

(event EventBeginPlay
  (Variables|Default|SetFrontViewLocation (Transformation|GetActorLocation))
  (bind _output_get (Variables|Default|SetCGGameMode (Class|CGLibrary|GetCGGameMode self)))
  (Utilities|IsValid _output_get
    (:Is%20Valid
      (EventDispatchers|AssignOnStartPlacingContainer (Variables|Default|GetCGGameMode) (delegate Custom|OnStartPlacingContainer_事件_0))
      (EventDispatchers|AssignOnEndPlacingContainer (Variables|Default|GetCGGameMode) (delegate Custom|OnEndPlacingContainer_事件_0))
      (EventDispatchers|AssignOnStartInspection (Variables|Default|GetCGGameMode) (delegate Custom|OnStartInspection_事件_0))
      (EventDispatchers|AssignOnEndInspection (Variables|Default|GetCGGameMode) (delegate Custom|OnEndInspection_事件_0)))))

(fn ConstructionScript)