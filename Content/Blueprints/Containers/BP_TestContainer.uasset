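; BP_TestContainer is a selectable container actor that shows its cost and a tilted, spinning unit preview.
; On BeginPlay a timeline animates its drop to the starting height, then marks it ready.
; During the player's container selection phase, team 0 containers lift and show cost text on hover, reversing when the cursor leaves.
; Releasing a click passes the container to the game mode to start placement, gated by the same macro check.
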(event OnBeginCursorOver(ContainerMesh)
  (params (TouchedComponent :type Primitive%20Component%20Object%20Reference))
  (bind _returnvalue (Transformation|GetActorLocation))
  (Utilities|RunifIsPlayerSelectingContainer
    (:Out
      (Rendering|SetVisibility (Variables|Default|GetTextRender) true false)
      (bind _zoffset (Timeline|ZOffset Play)
        (:Update
          (Transformation|SetActorLocation (Math|Vector|MakeVector (.x _returnvalue) (.y _returnvalue) (+ _zoffset (Variables|Default|GetStartingZPos))) false false))))))

(event OnEndCursorOver(ContainerMesh)
  (params (TouchedComponent :type Primitive%20Component%20Object%20Reference))
  (bind _returnvalue (Transformation|GetActorLocation))
  (Utilities|RunifIsPlayerSelectingContainer
    (:Out
      (Rendering|SetVisibility (Variables|Default|GetTextRender) false false)
      (bind _zoffset (Timeline|ZOffset Reverse)
        (:Update
          (Transformation|SetActorLocation (Math|Vector|MakeVector (.x _returnvalue) (.y _returnvalue) (+ _zoffset (Variables|Default|GetStartingZPos))) false false))))))

(event OnReleased(ContainerMesh)
  (params (TouchedComponent :type Primitive%20Component%20Object%20Reference) (ButtonReleased :type Key%20Structure))
  (bind _self self)
  (bind _returnvalue (Class|CGLibrary|GetCGGameMode _self))
  (Utilities|RunifIsPlayerSelectingContainer
    (:Out
      (Utilities|IsValid _returnvalue
        (:Is%20Valid
          (Class|CGGameMode|StartPlacingContainer _returnvalue self))))))

(event EventBeginPlay
  (bind _returnvalue (Transformation|GetActorLocation))
  (|CallParentFunction)
  (Utilities|FlowControl|Sequence
    (:then_0
      (Variables|Default|SetStartingZPos (.z (Transformation|GetActorLocation)))
      (Transformation|SetWorldRotation (Variables|Default|GetUnitPreviewMesh) (Math|Rotator|MakeRotator -2e+01 0.0 (Math|Random|RandomFloatinRange 0.0 3.6e+02)) false false)
      (bind _containerdropzpos (Timeline|ContainerSpawn PlayFromStart)
        (:Update
          (Transformation|SetActorLocation (Math|Vector|MakeVector (.x _returnvalue) (.y _returnvalue) (+ (* _containerdropzpos (Variables|Default|GetContainerStartingHeight)) (Variables|Default|GetStartingZPos))) false false))
        (:Finished
          (Variables|Default|SetIsReady true))))
    (:then_1
      (Rendering|Components|TextRender|SetText (Variables|Default|GetTextRender) (Utilities|Text|ToText(String) (Utilities|String|Append (Utilities|String|MakeLiteralString "Cost: ") (Utilities|String|ToString(Integer) (Variables|Default|GetCost))))))))

(event EventTick
  (params (DeltaSeconds :type Float%20%28single-precision%29))
  (Transformation|AddWorldRotation (Variables|Default|GetUnitPreviewMesh) (Math|Rotator|MakeRotator 0.0 0.0 (* DeltaSeconds 3e+01)) false false))

(fn ConstructionScript)