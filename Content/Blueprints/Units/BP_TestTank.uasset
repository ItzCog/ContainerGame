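; Test tank unit for a game with phased, action-based units, extending a parent unit's Move and Attack actions.
; Move approaches the target from FindTarget via BPCUnitMove; Attack turns and fires a projectile when in range.
; FinishAction follows movement completion, delayed projectile destruction, or a failed check.
; It also drives a health widget, hover indicator and debug target line while inspecting, click removal for nonzero teams, and a destruction explosion.
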(event OnBeginCursorOver(Capsule)
  (params (TouchedComponent :type Primitive%20Component%20Object%20Reference))
  (bind _returnvalue (Transformation|GetActorLocation))
  (bind _targetunit (Variables|Default|GetTargetUnit))
  (bind _returnvalue_2 (Transformation|GetActorLocation _targetunit))
  (if (Utilities|Enum|Equal(Enum) (Class|CGGameMode|GetGamePhase (Class|CGLibrary|GetCGGameMode self)) "PlayerInspecting")
    (Rendering|SetVisibility (Variables|Default|GetSelectionIndicator) true false)
    (Utilities|IsValid _targetunit
      (:Is%20Valid
        (if (<= (Math|Vector|Distance(Vector) _returnvalue _returnvalue_2) 8e+01)
          (Rendering|Debug|DrawDebugLine _returnvalue _returnvalue_2 "(R=1.000000,G=0.000000,B=0.000000,A=1.000000)" 3.0 0.0)
          (else
            (Rendering|Debug|DrawDebugLine _returnvalue _returnvalue_2 "(R=1.000000,G=0.000000,B=1.000000,A=1.000000)" 3.0 0.0)))))))

(event OnEndCursorOver(Capsule)
  (params (TouchedComponent :type Primitive%20Component%20Object%20Reference))
  (if (Utilities|Enum|Equal(Enum) (Class|CGGameMode|GetGamePhase (Class|CGLibrary|GetCGGameMode self)) "PlayerInspecting")
    (Rendering|SetVisibility (Variables|Default|GetSelectionIndicator) false false)))

(event Custom|OnProjectileDestroy_事件_0
  (Utilities|FlowControl|Delay 0.5)
  (Class|Unit|FinishAction))

(event Custom|OnCompletedMoving_事件_0
  (Class|Unit|FinishAction))

(event EventDestroyed
  (Niagara|SpawnSystematLocation "/Game/Assets/VFX/NS_TestExplosion.NS_TestExplosion" (Transformation|GetActorLocation)))

(event EventFinishPlacement
  (|CallParentFunction)
  (Rendering|SetVisibility (Variables|Default|GetSelectionIndicator) false false))

(event Game|Damage|EventAnyDamage
  (params (Damage :type Float%20%28single-precision%29) (DamageType :type Damage%20Type%20Object%20Reference) (InstigatedBy :type Controller%20Object%20Reference) (DamageCauser :type Actor%20Object%20Reference))
  (Default|CallOnHealthChanged0 (Variables|Default|GetHealth)))

(event EventMove
  (|CallParentFunction)
  (bind _returnvalue (Class|FindTarget|GetTargetUnit (Variables|Default|GetFindTarget)))
  (bind _output_get (Variables|Default|SetTargetUnit _returnvalue))
  (Utilities|IsValid _output_get
    (:Is%20Valid
      (Default|MovetoLocation (Variables|Default|GetBPC_UnitMove) (Transformation|GetActorLocation (Variables|Default|GetTargetUnit)) 6e+01 85.0))
    (:Is%20Not%20Valid
      (Class|Unit|FinishAction))))

(event EventAttack
  (bind _returnvalue (Transformation|GetActorLocation))
  (bind _self self)
  (bind _projectilespawner (Variables|Default|GetProjectileSpawner))
  (bind _targetunit (Variables|Default|GetTargetUnit))
  (bind _returnvalue_2 (Transformation|GetActorLocation _targetunit))
  (bind _returnvalue_3 (- _returnvalue_2 _returnvalue))
  (|CallParentFunction)
  (if (<= (Math|Vector|VectorLength _returnvalue_3) 9e+01)
    (Transformation|SetActorRotation (Math|Rotator|MakeRotator 0.0 0.0 (.yaw (Math|Rotator|MakeRotfromX _returnvalue_3))))
    (Class|CGLibrary|SpawnProjectile _self "/Game/Blueprints/Projectiles/BP_TestProjectile.BP_TestProjectile_C" (Math|Transform|MakeTransform (Transformation|GetWorldLocation _projectilespawner) (Transformation|GetWorldRotation _projectilespawner) "1,1,1") (Variables|Default|GetTeamID) _self (delegate Custom|OnProjectileDestroy_事件_0))
    (else
      (Class|Unit|FinishAction))))

(event EventBeginPlay
  (|CallParentFunction)
  (bind _aswbp_unit_health_display (Utilities|Casting|CastToWBP_UnitHealthDisplay (UserInterface|GetWidget (Variables|Default|GetHealthDisplay))))
  (Variables|/Game/Blueprints/UI/WBP_UnitHealthDisplay.WBP_UnitHealthDisplay_C|SetOwnerUnit _aswbp_unit_health_display self)
  (EventDispatchers|AssignOnCompletedMoving (Variables|Default|GetBPC_UnitMove) (delegate Custom|OnCompletedMoving_事件_0)))

(event MouseInput|EventActorOnClicked
  (params (ButtonPressed :type Key%20Structure :default "None"))
  (bind _self self)
  (if (!= (Variables|Default|GetTeamID) 0)
    (Class|CGGameMode|RemoveUnit (Class|CGLibrary|GetCGGameMode _self) _self)
    (Actor|DestroyActor)))

(fn ConstructionScript
  (Transformation|AttachComponentToComponent (Variables|Default|GetBarrel) (Variables|Default|GetSkeletalMesh) "TankBarrel" "KeepRelative" "KeepRelative" "KeepWorld" true))