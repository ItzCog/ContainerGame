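; Unit movement component that sends its owning pawn to a destination with a cap on how far it can travel.
; MoveToLocation resets the distance counter and starts an AI MoveTo with the given stopping distance.
; Tick sums the distance covered between frames and stops the AI controller's movement once the total exceeds the maximum, so the cap applies to the travelled path rather than straight-line distance.
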(event Custom|MoveToLocation
  (params (Destination :type Vector) (MaxMovingDistance :type Float%20%28single-precision%29) (StoppingDistance :type Float%20%28single-precision%29))
  (bind _returnvalue (Components|GetOwner))
  (bind _aspawn (Utilities|Casting|CastToPawn _returnvalue))
  (Variables|Default|SetOwnerLastFrameLocation (Transformation|GetActorLocation _returnvalue))
  (Variables|Default|SetMaxMovingDistance MaxMovingDistance)
  (Variables|Default|SetCumulativeDistance 0.0)
  (Variables|Default|SetbShouldMove true)
  (AI|AIMoveTo _aspawn Destination 0 StoppingDistance false))

(event EventTick
  (params (DeltaSeconds :type Float%20%28single-precision%29))
  (bind _returnvalue (Components|GetOwner))
  (bind _returnvalue_2 (Transformation|GetActorLocation _returnvalue))
  (if (Variables|Default|GetbShouldMove)
    (Variables|Default|SetCumulativeDistance (+ (Variables|Default|GetCumulativeDistance) (Math|Vector|Distance(Vector) (Variables|Default|GetOwnerLastFrameLocation) _returnvalue_2)))
    (Variables|Default|SetOwnerLastFrameLocation _returnvalue_2)
    (if (> (Variables|Default|GetCumulativeDistance) (Variables|Default|GetMaxMovingDistance))
      (Variables|Default|SetbShouldMove false)
      (AI|Navigation|StopMovement (AI|GetAIController (Components|GetOwner))))))