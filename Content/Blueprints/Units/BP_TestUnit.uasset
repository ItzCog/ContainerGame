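; Test unit Blueprint that performs move and attack actions, each ending in FinishAction.
; Move picks a target through FindTarget and takes a short AI step toward it.
; Attack turns to face the stored target, fires a team-tagged projectile and finishes shortly after that projectile is destroyed.
; It also links a health widget, shows hover selection and target debug during PlayerInspecting, and spawns an explosion when destroyed.
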(event OnBeginCursorOver(Capsule)
  (params (TouchedComponent :type Primitive%20Component%20Object%20Reference))
  (bind _targetunit (Variables|Default|GetTargetUnit))
  (if (Utilities|Enum|Equal(Enum) (Class|CGGameMode|GetGamePhase (Class|CGLibrary|GetCGGameMode self)) "PlayerInspecting")
    (Rendering|SetVisibility (Variables|Default|GetSelectionIndicator) true false)
    (Utilities|IsValid _targetunit
      (:Is%20Valid
        (Rendering|Debug|DrawDebugSphere (Transformation|GetActorLocation _targetunit) 1e+01 12 "(R=1.000000,G=1.000000,B=1.000000,A=1.000000)" 3.0 1.0)))))

(event OnEndCursorOver(Capsule)
  (params (TouchedComponent :type Primitive%20Component%20Object%20Reference))
  (if (Utilities|Enum|Equal(Enum) (Class|CGGameMode|GetGamePhase (Class|CGLibrary|GetCGGameMode self)) "PlayerInspecting")
    (Rendering|SetVisibility (Variables|Default|GetSelectionIndicator) false false)))

(event Custom|OnProjectileDestroy_事件_0
  (Utilities|FlowControl|Delay 0.5)
  (Class|Unit|FinishAction))

(event EventDestroyed
  (Niagara|SpawnSystematLocation "/Game/Assets/VFX/NS_TestExplosion.NS_TestExplosion" (Transformation|GetActorLocation) "0,0.000000, 0"))

(event EventFinishPlacement
  (|CallParentFunction)
  (Rendering|SetVisibility (Variables|Default|GetSelectionIndicator) false false))

(event Game|Damage|EventAnyDamage
  (params (Damage :type Float%20%28single-precision%29) (DamageType :type Damage%20Type%20Object%20Reference) (InstigatedBy :type Controller%20Object%20Reference) (DamageCauser :type Actor%20Object%20Reference))
  (Default|CallOnHealthChanged0 (Variables|Default|GetHealth)))

(event EventMove
  (bind _returnvalue (Transformation|GetActorLocation))
  (|CallParentFunction)
  (bind _returnvalue_2 (Class|FindTarget|GetTargetUnit (Variables|Default|GetFindTarget)))
  (bind _output_get (Variables|Default|SetTargetUnit _returnvalue_2))
  (AI|AIMoveTo self (+ (* (Math|Vector|Normalize (- (Transformation|GetActorLocation _output_get) _returnvalue)) 1e+01) _returnvalue) 0 5.0 false
    (:OnSuccess
      _)
    (:OnFail
      _))
  (Class|Unit|FinishAction))

(event EventAttack
  (bind _self self)
  (bind _projectilespawner (Variables|Default|GetProjectileSpawner))
  (|CallParentFunction)
  (Transformation|SetActorRotation (Math|Rotator|MakeRotator 0.0 0.0 (.yaw (Math|Rotator|MakeRotfromX (- (Transformation|GetActorLocation (Variables|Default|GetTargetUnit)) (Transformation|GetActorLocation))))))
  (bind _returnvalue (Class|CGLibrary|SpawnProjectile _self "/Game/Blueprints/Projectiles/BP_TestProjectile.BP_TestProjectile_C" (Math|Transform|MakeTransform (Transformation|GetWorldLocation _projectilespawner) (Transformation|GetWorldRotation _projectilespawner) "1,1,1") (Variables|Default|GetTeamID) _self))
  (EventDispatchers|AssignOnProjectileDestroy _returnvalue (delegate Custom|OnProjectileDestroy_事件_0)))

(event EventBeginPlay
  (|CallParentFunction)
  (bind _aswbp_unit_health_display (Utilities|Casting|CastToWBP_UnitHealthDisplay (UserInterface|GetWidget (Variables|Default|GetHealthDisplay))))
  (Variables|/Game/Blueprints/UI/WBP_UnitHealthDisplay.WBP_UnitHealthDisplay_C|SetOwnerUnit _aswbp_unit_health_display self))

(fn ConstructionScript)