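; BP_TestBase is a test unit Blueprint with placeholder actions and cursor-hover inspection.
; Its Move and Attack events immediately call FinishAction without doing any other work.
; During the game mode's PlayerInspecting phase, hovering over the capsule prints the unit's Health and shows SelectionIndicator.
; When the cursor leaves during that phase, the indicator is hidden again.
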(event OnBeginCursorOver(Capsule)
  (params (TouchedComponent :type Primitive%20Component%20Object%20Reference))
  (if (Utilities|Enum|Equal(Enum) (Class|CGGameMode|GetGamePhase (Class|CGLibrary|GetCGGameMode self)) "PlayerInspecting")
    (Development|PrintString (Utilities|String|Append "" "Health: " (Utilities|String|ToString(Integer) (Variables|Default|GetHealth))) true true "(R=0.000000,G=1.000000,B=0.200000,A=1.000000)")
    (Rendering|SetVisibility (Variables|Default|GetSelectionIndicator) true false)))

(event OnEndCursorOver(Capsule)
  (params (TouchedComponent :type Primitive%20Component%20Object%20Reference))
  (if (Utilities|Enum|Equal(Enum) (Class|CGGameMode|GetGamePhase (Class|CGLibrary|GetCGGameMode self)) "PlayerInspecting")
    (Rendering|SetVisibility (Variables|Default|GetSelectionIndicator) false false)))

(event EventMove
  (Class|Unit|FinishAction))

(event EventAttack
  (Class|Unit|FinishAction))

(fn ConstructionScript)