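; Test turret unit for a phase-based game: it stays put during Move and fires projectiles at a found target within a short range.
; Attack yaws toward the target and spawns a projectile, ending the action shortly after its destruction, or immediately if out of range.
; Hovering during the inspection phase shows the selection indicator and a range-colored debug line to any valid target.
; It also feeds a health widget and spawns a Niagara explosion when destroyed.
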(event OnBeginCursorOver(Capsule)
  (params (TouchedComponent :type Primitive%20Component%20Object%20Reference))
  (bind _returnvalue (Transformation|GetActorLocation))
  (bind _targetunit (Variables|Default|GetTargetUnit))
  (bind _returnvalue_2 (Transformation|GetActorLocation _targetunit))
  (if (Utilities|Enum|Equal(Enum) (Class|CGGameMode|GetGamePhase (Class|CGLibrary|GetCGGameMode self)) "PlayerInspecting")
    (Rendering|SetVisibility (Variables|Default|GetSelectionIndicator) true false)
    (Utilities|IsValid _targetunit
      (:Is%20Valid
        (if (<= (Math|Vector|Distance(Vector) _returnvalue _returnvalue_2) 1e+02)
          (Rendering|Debug|DrawDebugLine _returnvalue _returnvalue_2 "(R=1.000000,G=0.000000,B=0.000000,A=1.000000)" 3.0 0.0)
          (else
            (Rendering|Debug|DrawDebugLine _returnvalue _returnvalue_2 "(R=1.000000,G=0.000000,B=1.000000,A=1.000000)" 3.0 0.0)))))))

(event OnEndCursorOver(Capsule)
  (params (TouchedComponent :type Primitive%20Component%20Object%20Reference))
  (if (Utilities|Enum|Equal(Enum) (Class|CGGameMode|GetGamePhase (Class|CGLibrary|GetCGGameMode self)) "PlayerInspecting")
    (Rendering|SetVisibility (Variables|Default|GetSelectionIndicator) false false)))

(event Custom|OnProjectileDestroy_事件_0
  (Utilities|FlowControl|Delay 0.5)
  (Class|Unit|FinishAction))

(event EventDestroyed
  (Niagara|SpawnSystematLocation "/Game/Assets/VFX/NS_TestExplosion.NS_TestExplosion" (Transformation|GetActorLocation)))

(event EventFinishPlacement
  (|CallParentFunction)
  (Rendering|SetVisibility (Variables|Default|GetSelectionIndicator) false false))

(event Game|Damage|EventAnyDamage
  (params (Damage :type Float%20%28single-precision%29) (DamageType :type Damage%20Type%20Object%20Reference) (InstigatedBy :type Controller%20Object%20Reference) (DamageCauser :type Actor%20Object%20Reference))
  (Default|CallOnHealthChanged0 (Variables|Default|GetHealth)))

(event EventMove
  (|CallParentFunction)
  (Class|Unit|FinishAction))

(event EventAttack
  (bind _self self)
  (|CallParentFunction)
  (bind _returnvalue (Class|FindTarget|GetTargetUnit (Variables|Default|GetFindTarget)))
  (bind _output_get (Variables|Default|SetTargetUnit _returnvalue))
  (if (<= (Math|Vector|VectorLength (- (Transformation|GetActorLocation _output_get) (Transformation|GetActorLocation))) 1e+02)
    (Transformation|SetActorRotation (Math|Rotator|MakeRotator 0.0 0.0 (.yaw (Math|Rotator|MakeRotfromX (- (Transformation|GetActorLocation _output_get) (Transformation|GetActorLocation))))))
    (Class|CGLibrary|SpawnProjectile _self "/Game/Blueprints/Projectiles/BP_TestTurretProjectile.BP_TestTurretProjectile_C" (Math|Transform|MakeTransform (Transformation|GetWorldLocation (Variables|Default|GetProjectileSpawner)) (Math|Rotator|MakeRotator 0.0 (.pitch (Math|Rotator|MakeRotfromX (- (Transformation|GetActorLocation _output_get) (Transformation|GetActorLocation)))) (.yaw (Math|Rotator|MakeRotfromX (- (Transformation|GetActorLocation _output_get) (Transformation|GetActorLocation))))) "1,1,1") (Variables|Default|GetTeamID) _self (delegate Custom|OnProjectileDestroy_事件_0))
    (else
      (Class|Unit|FinishAction))))

(event EventBeginPlay
  (|CallParentFunction)
  (bind _aswbp_unit_health_display (Utilities|Casting|CastToWBP_UnitHealthDisplay (UserInterface|GetWidget (Variables|Default|GetHealthDisplay))))
  (Variables|/Game/Blueprints/UI/WBP_UnitHealthDisplay.WBP_UnitHealthDisplay_C|SetOwnerUnit _aswbp_unit_health_display self))

(fn ConstructionScript)