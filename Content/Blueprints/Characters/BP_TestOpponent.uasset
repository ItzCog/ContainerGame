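; BP_TestOpponent is a test AI opponent that deploys units on its turn through game mode events.
; Its energy is set to the new turn number when battling ends, and each deployment leaves it unchanged.
; On its turn, it randomly picks affordable team 1 Containers, spawns their units at random positions and frees their slots.
; It then destroys the used Containers and ends the turn after a short delay.
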(event Custom|OnStartOpponentTurn_事件_0
  (CallFunction|DeployUnit)
  (Utilities|FlowControl|Delay 1.0)
  (Class|CGGameMode|EndOpponentTurn (Class|CGLibrary|GetCGGameMode self)))

(event Custom|OnEndBattling_事件_0
  (params (NewTurnNumber :type Integer))
  (Variables|Default|SetRemainingEnergy NewTurnNumber))

(event EventBeginPlay
  (bind _self self)
  (bind _returnvalue (Class|CGLibrary|GetCGGameMode _self))
  (EventDispatchers|AssignOnStartOpponentTurn _returnvalue (delegate Custom|OnStartOpponentTurn_事件_0))
  (EventDispatchers|AssignOnEndBattling _returnvalue (delegate Custom|OnEndBattling_事件_0)))

(fn ConstructionScript)

(fn DeployUnit
  (Utilities|FlowControl|Sequence
    (:then_0
      (LocalVariables|SetUsedContainers (Utilities|Array|MakeArray 0))
      (bind _outactors (Actor|GetAllActorsOfClass "/Script/ContainerGame.Container"))
      (for _array_element _outactors
        (LocalVariables|SetCurrentContainer _array_element)
        (if (Math|Boolean|ANDBoolean (== (Variables|/Script/ContainerGame.Container|GetTeamID (LocalVariables|GetCurrentContainer)) 1) (<= (Variables|/Script/ContainerGame.Container|GetCost (LocalVariables|GetCurrentContainer)) (Variables|Default|GetRemainingEnergy)) (== (Math|Random|RandomIntegerinRange 1 3) 1))
          (Development|PrintString (Utilities|GetDisplayName (LocalVariables|GetCurrentContainer)))
          (Variables|Default|SetPlacementLocation (Math|Vector|MakeVector (Math|Random|RandomFloatinRange 3e+01 1.3e+02) (Math|Random|RandomFloatinRange -1.1e+02 1.1e+02) 115.0))
          (Class|CGWorldSettings|UnoccupyLocationforContainer (Class|CGLibrary|GetCGWorldSettings self) (LocalVariables|GetCurrentContainer))
          (bind _returnvalue (Game|SpawnActorfromClass (Variables|/Script/ContainerGame.Container|GetUnit (LocalVariables|GetCurrentContainer)) (Math|Transform|MakeTransform (Variables|Default|GetPlacementLocation) "0,180.000000, 0" "1,1,1") "Undefined" 0 0))
          (Variables|/Script/ContainerGame.Unit|SetTeamID _returnvalue 1)
          (Class|Unit|FinishPlacement _returnvalue)
          (Utilities|Array|Add (LocalVariables|GetUsedContainers) (LocalVariables|GetCurrentContainer)))))
    (:then_1
      (for _array_element_2 (LocalVariables|GetUsedContainers)
        (Actor|DestroyActor _array_element_2)))))